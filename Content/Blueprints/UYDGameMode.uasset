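; Game mode that handles player respawn, score tracking and timed zombie spawning.
; On begin play it starts a looping timer on the first EnemySpawner, calling SpawnEnemy at a rate set by EnemiesPerSecond.
; PlayerRespawn destroys all MainCharacters, spawns a new one at PlayerSpawn and possesses it, while incrementScore adds to Score.
; ZombieRespawn is an empty stub, and a loop that destroys all BaseEnemy actors is left unconnected.
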(event Custom|PlayerRespawn
  ;[1 1 1] Player Respawn
  (bind _outactors (Actor|GetAllActorsOfClass "/Game/Blueprints/Characters/MainCharacter.MainCharacter_C"))
  (for _array_element _outactors
    (Actor|DestroyActor _array_element))
  (bind _returnvalue (Game|SpawnActorfromClass "/Game/Blueprints/Characters/MainCharacter.MainCharacter_C" (Variables|Default|GetPlayerSpawn) false 0 0))
  (Pawn|Possess (Game|GetPlayerController 0) _returnvalue))

(event Custom|incrementScore
  (params (ScoreAmount :type Integer))
  ;[1 1 1] Score
  (Variables|Default|SetScore (+ ScoreAmount (Variables|Default|GetScore))))

(event Custom|ZombieRespawn)

(event EventTick
  (params (DeltaSeconds :type Float%20%28single-precision%29)))

(event EventBeginPlay
  ;[1 1 1] Spawn Zombies from the Spawner Collision Box every x amount of time
  (bind _outactors (Actor|GetAllActorsOfClass "/Game/Blueprints/Enemy/EnemySpawner.EnemySpawner_C"))
  (bind _output_get (Variables|Default|SetSpawner (Utilities|Array|Get(acopy) _outactors)))
  (Utilities|Time|SetTimerbyFunctionName _output_get "SpawnEnemy" (/ 1.0 (Variables|Default|GetEnemiesPerSecond)) true))

(fn ConstructionScript)