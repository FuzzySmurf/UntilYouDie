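; Base player character Blueprint handling weapon swapping, reloading, health and respawn, plus HUD creation.
; Q/E swaps go through PlayerWeaponManager to the weapon child actor, while R plays character and handgun reload animations.
; Handgun fire events toggle a looping timer that spawns bullets, muzzle flash and sound, but their calls here are unwired.
; Damage feeds HealthBase, with death triggering a delayed GameMode respawn; replicated-weapon functions are mostly empty stubs.
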(event Custom|HandgunFire
  ;[1 1 1] When Left click is pressed shoots continually untill released (reason is the way i was imagining the weapon fire mechanism to work on tablets is on the right side where our aming sircle will be when the player has his thumb on it he will aim at the location his thumb is located. Something like a thumbstick on an xbox/playstation controller)
  (Utilities|Time|SetTimerbyFunctionName 0 "HandgunConFire" 0.2 true)
  (Development|PrintString "AIM")
  (Variables|Attributes|SetIsShooting? true)
  (bind _ashandgun (Utilities|Casting|CastToHandgun (Variables|/Script/Engine.ChildActorComponent|GetChildActor (Variables|Default|GetHundgun))))
  (Default|FireWeapon _ashandgun))

(event Custom|HandgunStop
  ;[1 1 1] When Left click is pressed shoots continually untill released (reason is the way i was imagining the weapon fire mechanism to work on tablets is on the right side where our aming sircle will be when the player has his thumb on it he will aim at the location his thumb is located. Something like a thumbstick on an xbox/playstation controller)
  (Utilities|Time|ClearTimerbyFunctionName 0 "HandgunConFire")
  (Development|PrintString "STOP" true true "(R=1.000000,G=0.134206,B=0.229912,A=1.000000)")
  (Variables|Attributes|SetIsShooting? false))

(event Custom|Reload
  ;[1 1 1] play reload animation when key R is pressed. For the character model (not the weapon animation)
  (Utilities|FlowControl|Sequence
    (:then_0
      (bind _asmain_character_anim_bp (Utilities|Casting|CastToMainCharacterAnim_BP (Components|SkeletalMesh|GetAnimInstance (Variables|Character|GetMesh))))
      (Default|Reload _asmain_character_anim_bp))
    (:then_1
      ;[1 1 1] Cast to Hangun BP and execute custom event HandgunReload to play the reload animation for the handgun
      (bind _ashandgun (Utilities|Casting|CastToHandgun (Variables|/Script/Engine.ChildActorComponent|GetChildActor (Variables|Default|GetHundgun))))
      (Default|HandgunReload _ashandgun))))

(event Game|Damage|EventAnyDamage
  (params (Damage :type Float%20%28single-precision%29) (DamageType :type Damage%20Type%20Object%20Reference) (InstigatedBy :type Controller%20Object%20Reference) (DamageCauser :type Actor%20Object%20Reference))
  (bind _healthbase (Variables|Default|GetHealthBase))
  ;[1 1 1] Take Damage from BaseEnemy BP
  (Default|TakeDamage _healthbase Damage)
  (Variables|Default|SetMCHealth (Variables|/Game/Blueprints/Attributes/HealthBase.HealthBase_C|GetHealthCurrent _healthbase))
  (if (Variables|/Game/Blueprints/Attributes/HealthBase.HealthBase_C|GetIsDead _healthbase)
    (Input|DisableInput (Game|GetPlayerController 0))
    (Utilities|FlowControl|Delay 2.0)
    (Default|PlayerRespawn (Variables|Default|GetGameMode))))

(event EventBeginPlay
  ;[1 1 1] Show HUD
  (Utilities|FlowControl|Sequence
    (:then_0
      (bind _returnvalue (UserInterface|CreateWidget "/Game/Blueprints/UI/PlayerCharacter_HUD.PlayerCharacter_HUD_C"))
      (UserInterface|Viewport|AddtoViewport _returnvalue 0))
    (:then_1
      (bind _asuydgame_mode (Utilities|Casting|CastToUYDGameMode (Game|GetGameMode)))
      (bind _output_get (Variables|Default|SetGameMode _asuydgame_mode))
      (Variables|/Game/Blueprints/UYDGameMode.UYDGameMode_C|SetPlayerSpawn _output_get (Transformation|GetActorTransform)))))

(event Input|ActionEvents|InputActionWeaponSwap_Right
  ;[1 1 1] Press Q and E to rotate weapons
  (:Pressed
    (bind _weapon (Default|NextWeaponRight (Variables|Default|GetPlayerWeaponManager) (Variables|Default|GetCurrentWeapon)))
    (bind _output_get (Variables|Default|SetCurrentWeapon _weapon))
    (Development|PrintString (Utilities|String|EnumtoString _output_get) true true "(R=0.990000,G=0.980000,B=1.000000,A=1.000000)")
    (bind _asbp_base_weapon (Utilities|Casting|CastToBP_BaseWeapon (Variables|/Script/Engine.ChildActorComponent|GetChildActor (Variables|Default|GetWeapon))))
    (Default|EquipWeapon _asbp_base_weapon (Variables|Default|GetCurrentWeapon))))

(event Input|ActionEvents|InputActionFire
  ;[1 1 1] When Left click is pressed shoots continually untill released (reason is the way i was imagining the weapon fire mechanism to work on tablets is on the right side where our aming sircle will be when the player has his thumb on it he will aim at the location his thumb is located. Something like a thumbstick on an xbox/playstation controller)
)

(event Input|ActionEvents|InputActionWeaponSwap_Left
  ;[1 1 1] Press Q and E to rotate weapons
  (:Pressed
    (bind _weapon (Default|NextWeaponLeft (Variables|Default|GetPlayerWeaponManager) (Variables|Default|GetCurrentWeapon)))
    (bind _output_get (Variables|Default|SetCurrentWeapon _weapon))
    (Development|PrintString (Utilities|String|EnumtoString _output_get) true true "(R=0.928008,G=0.914560,B=1.000000,A=1.000000)")
    (bind _asbp_base_weapon (Utilities|Casting|CastToBP_BaseWeapon (Variables|/Script/Engine.ChildActorComponent|GetChildActor (Variables|Default|GetWeapon))))
    (Default|EquipWeapon _asbp_base_weapon (Variables|Default|GetCurrentWeapon))))

(event Input|KeyboardEvents|R
  ;[1 1 1] play reload animation when key R is pressed. For the character model (not the weapon animation)
  (:Pressed
    (CallFunction|Reload)))

(fn ConstructionScript
  (Class|SceneComponent|Attachto (Variables|Default|GetHundgun) (Variables|Character|GetMesh) "HandGunSocket" "SnapToTarget" true))

(fn HandgunConFire
  (bind _ashandgun (Utilities|Casting|CastToHandgun (Variables|/Script/Engine.ChildActorComponent|GetChildActor (Variables|Default|GetHundgun))))
  (Audio|PlaySoundatLocation "/Game/Sounds/9mm_Glock_17-SoundBible.9mm_Glock_17-SoundBible" "0, 0, 0")
  (bind _returnvalue (Effects|SpawnEmitterAttached "/Game/Particles/P_MuzzleFlash.P_MuzzleFlash" (Variables|/Game/Blueprints/Weapons/Handgun.Handgun_C|GetG19 _ashandgun) "MuzzleFlAsh" (Transformation|GetSocketLocation (Variables|/Game/Blueprints/Weapons/Handgun.Handgun_C|GetG19 _ashandgun) "MuzzleFlash") "0, 0, 0" "KeepWorldPosition"))
  (Transformation|SetRelativeScale3D _returnvalue "2.000000,2.000000,2.000000")
  (Game|SpawnActorfromClass "/Game/Blueprints/Weapons/Bullet_BP.Bullet_BP_C" (Math|Transform|MakeTransform (Transformation|GetSocketLocation (Variables|/Game/Blueprints/Weapons/Handgun.Handgun_C|GetG19 _ashandgun) "MuzzleFlash") (Transformation|GetActorRotation (Game|GetPlayerCharacter 0)) "1,1,1.000000") false 0 0))

(fn CalculateHealth
  (params (Amount :type Float%20%28single-precision%29))
  (Variables|Default|SetMCHealth (+ Amount (Variables|Default|GetMCHealth))))

(fn OnRepPrimaryWeapon)

(fn OnRepSecondaryWeapon)

(fn FirePrimaryWeapon)

(fn FireSecondaryWeapon)

(fn GiveDefaultPrimaryWeapon
  (bind _self self)
  (Networking|SwitchHasAuthority
    (:Authority
      (bind _returnvalue (Game|SpawnActorfromClass "/Game/Blueprints/Weapons/BPC_InstantHitWeapon.BPC_InstantHitWeapon_C" (Transformation|GetSocketTransform (Variables|Character|GetMesh) "HandGunSocket" "RTS_World") false _self _self))
      (bind _output_get (Variables|Weapons|SetPrimaryWeapon _returnvalue))
      (Class|Actor|AttachRootComponentto _output_get (Variables|Character|GetMesh) "HandGunSocket" "KeepWorldPosition" true))))