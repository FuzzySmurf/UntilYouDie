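; PlayerWeaponManager tracks the weapons a player owns and handles weapon pickups.
; PickedUpWeapon checks AllWeaponsOwned, adding new weapons to that array and routing owned ones to GetAmmoFromWeapon, with a debug print for each case.
; GetAmmoFromWeapon is an empty stub, so duplicate pickups grant no ammo here.
; NextWeapon and PreviousWeapon return the neighbor of a given weapon in the array, wrapping at either end.
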(event Custom|PickedUpWeapon
  (params (PickedUpWeapon :type Base%20Weapon%20Object%20Reference))
  ;[1 1 1] Handles all Weapon Pick-Ups
  (bind _ownweapon (CallFunction|DoWeOwnWeapon PickedUpWeapon))
  (if _ownweapon
    (CallFunction|GetAmmofromWeapon PickedUpWeapon)
    (Development|PrintString "Picking Up Weapon Ammo!")
    (else
      (CallFunction|AddWeapontoInventory PickedUpWeapon)
      (Development|PrintString "Added a new Weapon to Inventory!!"))))

(event EventTick
  (params (DeltaSeconds :type Float%20%28single-precision%29)))

(event EventBeginPlay)

(fn DoWeOwnWeapon
  (params (Weapon :type Base%20Weapon%20Object%20Reference))
  (LocalVariables|SetWeap Weapon)
  (bind _array_element (Utilities|Array|ForEachLoopwithBreak (Variables|Default|GetAllWeaponsOwned) :!label _label)
    (:LoopBody
      (if (== _array_element (LocalVariables|GetWeap))
        (LocalVariables|SetbMatch true)
        (goto _label Break)))
    (:Completed
      (return (LocalVariables|GetbMatch)))))

(fn AddWeapontoInventory
  (params (WeaponToAdd :type Base%20Weapon%20Object%20Reference))
  (Utilities|Array|Add (Variables|Default|GetAllWeaponsOwned) WeaponToAdd))

(fn GetAmmofromWeapon
  (params (Weapon :type Base%20Weapon%20Object%20Reference)))

(fn NextWeapon
  (params (CurrentWeapon :type Base%20Weapon%20Object%20Reference))
  (LocalVariables|SetcurWeap CurrentWeapon)
  (LocalVariables|SetweaponsIndexMax (- (Utilities|Array|Length (Variables|Default|GetAllWeaponsOwned)) 1))
  (bind _output_get (LocalVariables|SetcurWeapIdx (Utilities|Array|FindItem (Variables|Default|GetAllWeaponsOwned) (LocalVariables|GetcurWeap))))
  (bind _output_get_2 (LocalVariables|SetnewWeapIdx (+ _output_get 1)))
  (if (> _output_get_2 (LocalVariables|GetweaponsIndexMax))
    (LocalVariables|SetnewWeapIdx 0))
  (bind _output_get_3 (LocalVariables|SetnewWeap (Utilities|Array|Get(acopy) (Variables|Default|GetAllWeaponsOwned) (LocalVariables|GetnewWeapIdx))))
  (return _output_get_3))

(fn PreviousWeapon
  (params (CurrentWeapon :type Base%20Weapon%20Object%20Reference))
  (LocalVariables|SetCurWeap CurrentWeapon)
  (LocalVariables|SetweaponsIdxMax (- (Utilities|Array|Length (Variables|Default|GetAllWeaponsOwned)) 1))
  (bind _output_get (LocalVariables|SetcurWeapIdx (Utilities|Array|FindItem (Variables|Default|GetAllWeaponsOwned) (LocalVariables|GetCurWeap))))
  (bind _output_get_2 (LocalVariables|SetnewWeapIdx (- _output_get 1)))
  (if (< _output_get_2 0)
    (LocalVariables|SetnewWeapIdx (LocalVariables|GetweaponsIdxMax)))
  (bind _output_get_3 (LocalVariables|SetnewWeap (Utilities|Array|Get(acopy) (Variables|Default|GetAllWeaponsOwned) (LocalVariables|GetnewWeapIdx))))
  (return _output_get_3))