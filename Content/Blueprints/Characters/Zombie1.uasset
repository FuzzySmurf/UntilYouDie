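; Zombie enemy Blueprint that chases the player on sight and otherwise wanders to random points.
; PawnSensing's OnSeePawn sets SeePlayer, casts the seen pawn to MainCharacter and runs AIMoveTo toward it.
; While SeePlayer is false, Tick issues random-point moves, using a Moving flag to prevent overlapping requests.
; SeePlayer clears only when the chase move succeeds, not when sight is lost or the move fails.
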(event OnSeePawn(PawnSensing)
  (params (Pawn :type Pawn%20Object%20Reference))
  ;[1 1 1] using PawnSensing component i can get OnSeePawn event so when the zombie sees the player will start to chase him
  (Variables|Default|SetbSeePlayer true)
  (bind _asmain_character (Utilities|Casting|CastToMainCharacter Pawn))
  (AI|AIMoveTo self "0, 0, 0" _asmain_character 5.0 false
    (:OnSuccess
      (Variables|Default|SetbSeePlayer false))))

(event EventTick
  (params (DeltaSeconds :type Float%20%28single-precision%29))
  ;[1 1 1] just an experiment when the zombie loses sight of the player will move randomly untill he sees the target
  (if (not (Variables|Default|GetbSeePlayer))
    (if (not (Variables|Default|GetbMoving))
      (AI|AIMoveTo self (Class|NavigationSystem|GetRandomPoint) 0 5.0 false
        (:then
          (Variables|Default|SetbMoving true))
        (:OnSuccess
          (Variables|Default|SetbMoving false :!label _label))
        (:OnFail
          (goto _label))))))

(fn ConstructionScript)