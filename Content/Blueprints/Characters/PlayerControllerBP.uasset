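; Player controller for a top-down shooter, translating input into main character movement, mouse aiming, firing, weapon swapping and respawn.
; Movement follows world axes, while Tick yaws the pawn toward the deprojected mouse position.
; Firing drives the primary weapon, delaying the shot when the current montage is inactive.
; Respawn calls UYDGameMode on authority only; the reload input only fetches the pawn, without reloading.
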(event EventTick
  (params (DeltaSeconds :type Float%20%28single-precision%29))
  (bind _returnvalue (Pawn|GetControlledPawn))
  ;[1 1 1] View Rotation
  (if (!= _returnvalue 0)
    (Transformation|SetActorRotation _returnvalue (Class|KismetMathLibrary|MakeRot 0.0 (.Yaw (Class|KismetMathLibrary|BreakRot (Math|Rotator|FindLookatRotation (Transformation|GetActorLocation _returnvalue) (.WorldLocation (Game|Player|ConvertMouseLocationToWorldSpace))))) 0.0))))

(event Input|ActionEvents|InputActionWeaponSwap_Left
  ;[1 1 1] Rotate to the next available weapon (Left)
  (:Pressed
    (bind _maincharacter (CallFunction|MainCharacterPawn))
    (Default|WeaponRotate _maincharacter true)))

(event Input|ActionEvents|InputActionWeaponSwap_Right
  ;[1 1 1] Rotate to the next available weapon (Right)
  (:Pressed
    (bind _maincharacter (CallFunction|MainCharacterPawn))
    (Default|WeaponRotate _maincharacter false)))

(event Input|ActionEvents|InputActionFire
  (bind _returnvalue (Game|GetPlayerCharacter 0))
  ;[1 1 1] Fire Primary Weapon
  (:Pressed
    (bind _maincharacter (CallFunction|MainCharacterPawn))
    (Variables|/Game/Blueprints/Characters/MainCharacter.MainCharacter_C|SetIsShooting? _maincharacter true)
    ;[1 0.424 0.05063] Delay the first shot of any weapon when in Hold Weapon Animation is active
    (bind _asmain_char_ab (Utilities|Casting|CastToMainChar_AB (Components|SkeletalMesh|GetAnimInstance (Variables|/Script/Engine.Character|GetMesh _returnvalue))))
    (bind _returnvalue_2 (Animation|GetCurrentMontage _returnvalue :!class /Script/Engine.Character))
    (bind _returnvalue_3 (Class|AnimInstance|MontageIsActive _asmain_char_ab _returnvalue_2))
    (if _returnvalue_3
      _
      (else
        (Utilities|FlowControl|Delay 0.2)))
    (Default|OnFire (Variables|/Game/Blueprints/Characters/MainCharacter.MainCharacter_C|GetPrimaryWeapon _maincharacter)))
  (:Released
    (Variables|/Game/Blueprints/Characters/MainCharacter.MainCharacter_C|SetIsShooting? _maincharacter false)
    (Default|ResetFiring (Variables|/Game/Blueprints/Characters/MainCharacter.MainCharacter_C|GetPrimaryWeapon _maincharacter))))

(event Input|ActionEvents|InputActionReloadWeapon
  (:Pressed
    (CallFunction|MainCharacterPawn)))

(event Input|ActionEvents|InputActionRespawn
  (bind _returnvalue (Game|GetGameMode))
  ;[1 1 1] Controlls the Trigger Respawn
  (:Pressed
    (Networking|SwitchHasAuthority
      (:Authority
        (Utilities|IsValid _returnvalue
          (:Is%20Valid
            (bind _asuydgame_mode (Utilities|Casting|CastToUYDGameMode _returnvalue))
            (Default|PlayerRespawn _asuydgame_mode self)))))))

(event Input|AxisEvents|InputAxisForward_Backward
  (params (AxisValue :type Float%20%28single-precision%29))
  ;[1 1 1] Movement
  (Pawn|Input|AddMovementInput (Pawn|GetControlledPawn) "1.000000, 0, 0" AxisValue false))

(event Input|AxisEvents|InputAxisLeft_Right
  (params (AxisValue :type Float%20%28single-precision%29))
  ;[1 1 1] Movement
  (Pawn|Input|AddMovementInput (Pawn|GetControlledPawn) "0.000000,1.000000, 0" AxisValue false))

(fn ConstructionScript)

(fn MainCharacterPawn
  (bind _returnvalue (Pawn|GetControlledPawn))
  (if (!= _returnvalue 0)
    (bind _asmain_character (Utilities|Casting|CastToMainCharacter _returnvalue)
      (:then
        (LocalVariables|SetmainChar _asmain_character))
      (:CastFailed
        (Development|PrintString "Cast To MainCharacter failed in PlayerControllerBP" true true "(R=1.000000,G=0.023529,B=0.976471,A=1.000000)")))
    (else
      (Development|PrintString "Could not find ControllerPawn in PlayerControllerBP" true true "(R=1.000000,G=0.023529,B=0.976471,A=1.000000)")))
  (return (LocalVariables|GetmainChar)))