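; Player controller that moves the controlled pawn along world axes and turns it toward the mouse cursor.
; Forward_Backward and Left_Right axis inputs feed movement input on fixed world X and Y, independent of pawn facing.
; Each tick, it sets the pawn's yaw from a look-at toward the deprojected mouse world location, with pitch and roll zeroed and no trace used.
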(event EventTick
  (params (DeltaSeconds :type Float%20%28single-precision%29))
  (bind _returnvalue (Pawn|GetControlledPawn))
  ;[1 1 1] View Rotation
  (Transformation|SetActorRotation _returnvalue (Class|KismetMathLibrary|MakeRot 0.0 (.Yaw (Class|KismetMathLibrary|BreakRot (Math|Rotator|FindLookatRotation (Transformation|GetActorLocation _returnvalue) (.WorldLocation (Game|Player|ConvertMouseLocationToWorldSpace))))) 0.0)))

(event Input|AxisEvents|InputAxisForward_Backward
  (params (AxisValue :type Float%20%28single-precision%29))
  ;[1 1 1] Movement
  (Pawn|Input|AddMovementInput (Pawn|GetControlledPawn) "1.000000, 0, 0" AxisValue false))

(event Input|AxisEvents|InputAxisLeft_Right
  (params (AxisValue :type Float%20%28single-precision%29))
  ;[1 1 1] Movement
  (Pawn|Input|AddMovementInput (Pawn|GetControlledPawn) "0,1.000000, 0" AxisValue false))

(fn ConstructionScript)