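; Handgun Blueprint for a Glock 19 that handles the feedback and line trace for firing a shot.
; The FireWeapon event plays a gunshot sound, attaches an enlarged muzzle flash at the muzzle socket and spawns a bullet particle at the ammo eject socket.
; It then runs a short forward visibility trace from the muzzle with debug drawing, and the hit result is not used.
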(event Custom|Fire%20Weapon
  (bind _g19 (Variables|Default|GetG19))
  (bind _g19_2 (Variables|Default|GetG19))
  (bind _returnvalue (Transformation|GetSocketLocation _g19_2 "MuzzleFlash"))
  (bind _returnvalue_2 (Transformation|GetSocketLocation _g19 "MuzzleFlAsh"))
  ;[1 1 1] After the Fire (left click) is pressed play sound and spawn particles
  (Audio|PlaySoundatLocation "/Game/Weapons/9mm_Glock_17-SoundBible.9mm_Glock_17-SoundBible" _returnvalue_2)
  (bind _returnvalue_3 (Effects|SpawnEmitterAttached "/Game/Particles/P_MuzzleFlash.P_MuzzleFlash" _g19 "MuzzleFlAsh" _returnvalue_2 "0, 0, 0" "KeepWorldPosition"))
  (Transformation|SetRelativeScale3D _returnvalue_3 "2.000000,2.000000,2.000000")
  (Effects|SpawnEmitteratLocation "/Game/Particles/P_BulletProjectile.P_BulletProjectile" (Transformation|GetSocketLocation _g19 "AmmoEject"))
  ;[1 1 1] Draw a trace of forward vector from the muzzleflash socket
  (Collision|LineTraceByChannel _returnvalue (+ (* (Math|Vector|GetForwardVector (Variables|Default|GetG19)) 1e+03) _returnvalue) "TraceTypeQuery1" false 0 "ForDuration"))

(fn ConstructionScript)