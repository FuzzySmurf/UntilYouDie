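; Base weapon Blueprint that handles firing, ammo checks and muzzle and impact effects on a skeletal mesh.
; OnFire checks ammo and plays socket-attached flash and sound, but hit detection always returns false and server verification and damage are empty stubs.
; A separate FireOffWeapon function spawns Bullet_BP projectiles using the player character's rotation.
; DecrementAmmo is never called here, AimWeapon's timer names no function, and DisableFiring only sets a flag.
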(event Custom|PlayMuzzleFlash
  (bind _returnvalue (Effects|SpawnEmitterAttached (Variables|Default|GetMuzzleFlashParticleSystem) (Variables|Default|GetSkeletalMesh) (Variables|Default|GetMuzzleSocket)))
  (Utilities|FlowControl|Delay 0.1)
  (Components|DestroyComponent _returnvalue))

(event Custom|OnFireDeactivate
  (CallFunction|DisableFiring))

(event Custom|ServerVerifyHitObjects)

(event Custom|OnFire
  ;[1 1 1] Used to Trigger Weapon
  (CallFunction|CanWeaponFire)
  (if (Variables|Default|GetcanFire)
    (CallFunction|AimWeapon)
    (CallFunction|PlayMuzzleFlash)
    (CallFunction|PlayFireSound)
    (bind _objecthit (CallFunction|DetermineHitObjects))
    (if _objecthit
      (CallFunction|ServerVerifyHitObjects)
      (CallFunction|ApplyDamagetoHitActors)
      (else
        (Development|PrintString "Didn't Hit Anything")))))

(event Custom|ApplyDamageToHitActors)

(event Custom|PlayFireSound
  (Class|GameplayStatics|PlaySoundAttached (Variables|Default|GetSfxFireWeapon) (Variables|Default|GetSkeletalMesh) (Variables|Default|GetMuzzleSocket)))

(event Custom|DisplayImpactEffect
  (params (HitLocation :type Vector) (HitRotation :type Rotator))
  (Effects|SpawnEmitteratLocation (Variables|Default|GetImpactEffect) HitLocation HitRotation))

(event Custom|PlayImpactSound
  (params (Location :type Vector))
  (Audio|PlaySoundatLocation (Variables|Default|GetImpactSound) Location))

(fn ConstructionScript)

(fn FireOffWeapon
  (bind _skeletalmesh (Variables|Default|GetSkeletalMesh))
  (bind _returnvalue (Transformation|GetSocketLocation _skeletalmesh "MuzzleFlash"))
  (bind _canweaponfire (CallFunction|CanWeaponFire))
  (if _canweaponfire
    (Audio|PlaySoundatLocation (Variables|Default|GetSfxFireWeapon) "0, 0, 0")
    (bind _returnvalue_2 (Effects|SpawnEmitterAttached "/Game/Particles/P_Muzzle_Flash.P_Muzzle_Flash" 0 "MuzzleFlAsh" _returnvalue "0, 0, 0" "KeepWorldPosition"))
    (Transformation|SetRelativeScale3D _returnvalue_2 "2.000000,2.000000,2.000000")
    (Game|SpawnActorfromClass "/Game/Blueprints/Weapons/Bullet_BP.Bullet_BP_C" (Math|Transform|MakeTransform _returnvalue (Transformation|GetActorRotation (Game|GetPlayerCharacter 0))) false 0 0)))

(fn AssignWeapon
  (params (WeaponToUse :type Skeletal%20Mesh%20Component%20Object%20Reference))
  (Variables|Default|SetSkeletalMesh WeaponToUse))

(fn CanWeaponFire
  (if (> (Variables|Ammo|GetammoCurrent) 0)
    (Variables|Default|SetcanFire true)
    (else
      (Variables|Default|SetcanFire false)))
  (return (Variables|Default|GetcanFire)))

(fn DecrementAmmo
  (if (> (Variables|Ammo|GetammoCurrent) 0)
    (Variables|Ammo|SetammoCurrent (- (Variables|Ammo|GetammoCurrent) 1))
    (else
      (Development|PrintString "out of ammo! Reload!"))))

(fn DetermineHitObjects
  (return false))

(fn AimWeapon
  (Utilities|Time|SetTimerbyFunctionName 0 "" 0.06))

(fn DisableFiring
  (Variables|Default|SetbreakFiringLoop true))