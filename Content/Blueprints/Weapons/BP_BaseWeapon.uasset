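; BP_BaseWeapon is a base weapon Blueprint that handles firing from the active weapon component.
; AssignWeapon sets WeaponInUse, which supplies the MuzzleFlash socket location for firing.
; FireOffWeapon plays a shot sound at world origin, spawns a scaled muzzle flash and spawns Bullet_BP at the socket, using player character 0's rotation.
; EquipWeapon is unfinished: its switch has empty branches and the G19 assignment is disconnected.
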(event EventBeginPlay)

(event Collision|EventActorBeginOverlap
  (params (OtherActor :type Actor%20Object%20Reference)))

(event EventTick
  (params (DeltaSeconds :type Float%20%28single-precision%29)))

(fn ConstructionScript)

(fn FireOffWeapon
  (bind _weaponinuse (Variables|Default|GetWeaponInUse))
  (bind _returnvalue (Transformation|GetSocketLocation _weaponinuse "MuzzleFlash"))
  (Audio|PlaySoundatLocation (Variables|Default|GetSfxShooting) "0, 0, 0")
  (bind _returnvalue_2 (Effects|SpawnEmitterAttached "/Game/Particles/P_MuzzleFlash.P_MuzzleFlash" 0 "MuzzleFlAsh" _returnvalue "0, 0, 0" "KeepWorldPosition"))
  (Transformation|SetRelativeScale3D _returnvalue_2 "2.000000,2.000000,2.000000")
  (Game|SpawnActorfromClass "/Game/Blueprints/Weapons/Bullet_BP.Bullet_BP_C" (Math|Transform|MakeTransform _returnvalue (Transformation|GetActorRotation (Game|GetPlayerCharacter 0))) false 0 0))

(fn AssignWeapon
  (params (WeaponToUse :type Skeletal%20Mesh%20Component%20Object%20Reference))
  (Variables|Default|SetWeaponInUse WeaponToUse))

(fn EquipWeapon
  (params (weapon :type WeaponEnum%20Enum))
  (switch Utilities|FlowControl|Switch|SwitchonWeaponEnum weapon))