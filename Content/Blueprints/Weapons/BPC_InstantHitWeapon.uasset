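; Hitscan weapon Blueprint that extends a parent weapon with instant line-trace hits.
; ServerVerifyHitObjects clears HitResults, then fires repeated, identical Camera-channel traces straight from the muzzle socket out to Range, storing each hit.
; ApplyDamagetoHitActors damages each stored actor, spawns an impact emitter and plays a sound.
; DetermineHitObjects duplicates the trace loop without clearing, returning a hit flag; traces draw persistent debug lines.
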(event EventDisplayImpactEffect
  (params (HitLocation :type Vector) (HitRotation :type Rotator))
  (Effects|SpawnEmitteratLocation (Variables|Default|GetImpactEffect) HitLocation HitRotation))

(event EventBeginPlay)

(event Collision|EventActorBeginOverlap
  (params (OtherActor :type Actor%20Object%20Reference)))

(event EventTick
  (params (DeltaSeconds :type Float%20%28single-precision%29)))

(event EventServerVerifyHitObjects
  (bind _self self)
  (bind _muzzlesocket (Variables|Default|GetMuzzleSocket))
  (bind _skeletalmesh (Variables|Default|GetSkeletalMesh _self))
  (bind _returnvalue (Transformation|GetSocketLocation _skeletalmesh _muzzlesocket))
  ;[1 1 1] Determine what objects are hit with a shot and add them to an array that is returned to fire event.
  (|CallParentFunction)
  (Utilities|Array|Clear (Variables|Default|GetHitResults))
  (for _index (range 0 (Variables|Default|GetTracesUsed))
    (bind (_outhit _returnvalue_2) (Collision|LineTraceByChannel _returnvalue (+ _returnvalue (* (Math|Vector|GetForwardVector (Transformation|GetSocketRotation _skeletalmesh _muzzlesocket)) (Variables|Default|GetRange))) "TraceTypeQuery2" false 0 "Persistent"))
    (if _returnvalue_2
      (bind _returnvalue_3 (Utilities|Array|Add (Variables|Default|GetHitResults) _outhit))
      (Development|PrintString (Utilities|String|BuildString(Object) (Utilities|String|ToString(Integer) _returnvalue_3) "Hit Actor: " 0)))))

(event EventApplyDamagetoHitActors
  (for _index (range 0 (- (Utilities|Array|Length (Variables|Default|GetHitResults)) 1))
    (Development|PrintString (Utilities|String|BuildString(Object) "" "Hit Object: " (.HitActor (Collision|BreakHitResult (Utilities|Array|Get(acopy) (Variables|Default|GetHitResults) _index)))))
    (Game|Damage|ApplyDamage (.HitActor (Collision|BreakHitResult (Utilities|Array|Get(acopy) (Variables|Default|GetHitResults) _index))) (Variables|Default|GetDamage) (Game|GetInstigatorController) self "/Script/Engine.DamageType")
    (CallFunction|DisplayImpactEffect (.Location (Collision|BreakHitResult (Utilities|Array|Get(acopy) (Variables|Default|GetHitResults) _index))) "0, 0, 0")
    (CallFunction|PlayImpactSound (.Location (Collision|BreakHitResult (Utilities|Array|Get(acopy) (Variables|Default|GetHitResults) _index))))))

(fn ConstructionScript
  (|CallParentFunction))

(fn DetermineHitObjects
  (bind _self self)
  (bind _muzzlesocket (Variables|Default|GetMuzzleSocket))
  (bind _skeletalmesh (Variables|Default|GetSkeletalMesh _self))
  (bind _returnvalue (Transformation|GetSocketLocation _skeletalmesh _muzzlesocket))
  (for _index (range 0 (Variables|Default|GetTracesUsed))
    (bind (_outhit _returnvalue_2) (Collision|LineTraceByChannel _returnvalue (+ _returnvalue (* (Math|Vector|GetForwardVector (Transformation|GetSocketRotation _skeletalmesh _muzzlesocket)) (Variables|Default|GetRange))) "TraceTypeQuery2" false 0 "Persistent"))
    (if _returnvalue_2
      (Utilities|Array|Add (Variables|Default|GetHitResults) _outhit)
      (LocalVariables|SetisObjectHit true)))
  (return (LocalVariables|GetisObjectHit)))