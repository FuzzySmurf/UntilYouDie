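; Handgun weapon Blueprint built around a G19 mesh, with reload and fire events that are only partly wired.
; HandgunReload prints debug strings and, when the Reload flag is set, plays a montage on the mesh's AnimInstance; otherwise it resets a DoOnce.
; FireWeapon is empty: the gunshot sound, muzzle flash, socket-based debug line trace and ammo-eject emitter nodes are disconnected and never run.
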(event Custom|Fire%20Weapon
  ;[1 1 1] After the Fire (left click) is pressed play sound and spawn particles
)

(event Custom|HandgunReload
  (Development|PrintString "Hello")
  (bind _output_get (Variables|Default|SetReload (Variables|Default|GetReload)))
  (if _output_get
    (Development|PrintString "play montage" true true "(R=1.000000,G=0.000000,B=0.018721,A=1.000000)")
    (Animation|Montage|MontagePlay (Components|SkeletalMesh|GetAnimInstance (Variables|Default|GetG19)) "/Game/Weapons/testweapon_Skeleton_Montage.testweapon_Skeleton_Montage" 1.0)
    (else
      (Utilities|FlowControl|DoOnce false) ; enters at Reset
    )))

(fn ConstructionScript)