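; Projectile weapon Blueprint that fires by spawning a projectile actor from the weapon's muzzle.
; OnFire checks CanWeaponFire and, when allowed, plays the muzzle flash and fire sound, then calls SpawnProjectile.
; SpawnProjectile spawns the configurable ProjectileType class at the skeletal mesh's muzzle socket world transform.
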(event Custom|SpawnProjectile
  ;[1 1 1] Spawn's Projectile @ Muzzle Socket Location
  (Game|SpawnActorfromClass (Variables|Default|GetProjectileType) (Transformation|GetSocketTransform (Variables|Default|GetSkeletalMesh self) (Variables|Default|GetMuzzleSocket) "RTS_World") false 0 0))

(event EventBeginPlay)

(event Collision|EventActorBeginOverlap
  (params (OtherActor :type Actor%20Object%20Reference)))

(event EventTick
  (params (DeltaSeconds :type Float%20%28single-precision%29)))

(event EventOnFire
  (CallFunction|CanWeaponFire)
  (if (Variables|Default|GetcanFire)
    (CallFunction|PlayMuzzleFlash)
    (CallFunction|PlayFireSound)
    (CallFunction|SpawnProjectile)))

(fn ConstructionScript
  (|CallParentFunction))