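; Beam projectile actor for weapons that damages whatever its collision sphere hits and explodes when destroyed.
; On a sphere hit it calls destroy on itself, prints the hit object as debug text, then applies its core damage, crediting the instigator's controller.
; The Destroyed event spawns the explosion emitter and sound at the sphere's location, so the effects accompany any destruction, not only impacts.
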(event OnComponentHit(SphereCollision)
  (params (OtherActor :type Actor%20Object%20Reference) (OtherComp :type Primitive%20Component%20Object%20Reference) (NormalImpulse :type Vector :default "0, 0, 0") (Hit :type Hit%20Result%20Structure%20%28by%20ref%29))
  (bind _hitactor (Collision|BreakHitResult Hit))
  (Actor|DestroyActor)
  (Development|PrintString (Utilities|String|BuildString(Object) "" "Hit Object: " _hitactor))
  (Game|Damage|ApplyDamage _hitactor (Variables|Default|GetCoreDamage) (Game|GetInstigatorController) self))

(event EventDestroyed
  (bind _self self)
  (bind _spherecollision (Variables|Default|GetSphereCollision _self))
  (bind _returnvalue (Transformation|GetWorldLocation _spherecollision))
  (Effects|SpawnEmitteratLocation (Variables|Default|GetExplosionEffect) _returnvalue)
  (Audio|PlaySoundatLocation (Variables|Default|GetExplosionSound) _returnvalue))

(event EventBeginPlay)

(event Collision|EventActorBeginOverlap
  (params (OtherActor :type Actor%20Object%20Reference)))

(event EventTick
  (params (DeltaSeconds :type Float%20%28single-precision%29)))

(fn ConstructionScript
  (|CallParentFunction))