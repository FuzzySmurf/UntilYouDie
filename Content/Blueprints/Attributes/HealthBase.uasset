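; HealthBase is a health attribute Blueprint that starts current health at its maximum on BeginPlay and provides a TakeDamage function.
; When damageable, TakeDamage sets health to the damage amount minus current health, the reverse of the usual subtraction.
; A result below zero destroys player character 0, whichever actor owns the health, while non-damageable instances only print a debug message.
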(event EventTick
  (params (DeltaSeconds :type Float%20%28single-precision%29)))

(event EventBeginPlay
  (Variables|Default|SetHealthCurrent (Variables|Default|GetHealthMax)))

(fn TakeDamage
  (params (DamageAmount :type Integer))
  ;[1 1 1] If Actor takes damage, it will lower current Damage of the Parent Actor.
  (if (Variables|Default|GetisDamageable)
    (bind _output_get (Variables|Default|SetHealthCurrent (- DamageAmount (Variables|Default|GetHealthCurrent))))
    (Math|Integer|CompareInt _output_get 0
      (:<
        (Development|PrintString "working")
        (Actor|DestroyActor (Game|GetPlayerCharacter 0))))
    (else
      (Development|PrintString "Cannot Take Damage" true true "(R=0.875000,G=0.043428,B=0.160834,A=1.000000)"))))