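; BaseEnemy is a zombie enemy Blueprint that damages the main character on overlap and can be killed for score.
; Incoming damage feeds its health component and triggers the anim Blueprint's hit reaction; death awards score, detaches the controller, disables collision and destroys it after a delay.
; Overlap plays an attack montage, applies damage and starts a looping timer without a function name.
; The construction script's mesh and material setup is unconnected.
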(event Collision|EventActorBeginOverlap
  (params (OtherActor :type Actor%20Object%20Reference))
  ;[1 1 1] Damage MainCharacter
  (bind _asmain_character (Utilities|Casting|CastToMainCharacter OtherActor))
  (bind _output_get (Variables|Default|SetMainCharacter _asmain_character))
  (Animation|PlayAnimMontage "/Game/Characters/Zombies/ZombieGroupA/anims/M_ZATTACK.M_ZATTACK" 1.0 "None")
  (Game|Damage|ApplyDamage OtherActor (Variables|Default|GetDamageToMC) 0 (Variables|Default|GetZombie))
  (Utilities|Time|SetTimerbyFunctionName _output_get "" (/ 1.0 2.0) true))

(event Collision|EventActorEndOverlap
  (params (OtherActor :type Actor%20Object%20Reference))
  ;[1 1 1] Damage MainCharacter
  (if (== OtherActor (Variables|Default|GetMainCharacter))
    (Utilities|Time|ClearTimerbyFunctionName 0 "")
    (Development|PrintString "clear timer")))

(event Game|Damage|EventAnyDamage
  (params (Damage :type Float%20%28single-precision%29) (DamageType :type Damage%20Type%20Object%20Reference) (InstigatedBy :type Controller%20Object%20Reference) (DamageCauser :type Actor%20Object%20Reference))
  ;[1 1 1] Take Damage
  (Development|PrintString (Utilities|String|ToString(Float) Damage))
  (Default|TakeDamage (Variables|Default|GetHealthBase) Damage)
  (Variables|Default|SetIsHit true)
  (bind _aszombie_ga_ab (Utilities|Casting|CastToZombie_GA_AB (Components|SkeletalMesh|GetAnimInstance (Variables|Character|GetMesh))))
  (Default|GetHit _aszombie_ga_ab)
  (if (<= (Variables|/Game/Blueprints/Attributes/HealthBase.HealthBase_C|GetHealthCurrent (Variables|Default|GetHealthBase)) 0.0)
    ;[1 1 1] If Dead disable collision and kill actor after 5 seconds
    (Variables|Default|SetIsDead true)
    (bind _asuydgame_mode (Utilities|Casting|CastToUYDGameMode (Game|GetGameMode)))
    (Default|IncrementScore _asuydgame_mode 200)
    (Class|Pawn|DetachfromControllerPendingDestroy)
    (Collision|SetCollisionResponsetoAllChannels (Variables|Collision|GetCapsuleComponent) "ECR_Ignore")
    (Utilities|FlowControl|Delay 5.0)
    (Actor|DestroyActor)))

(fn ConstructionScript
  ;[1 1 1] Sets an Enemy Mesh, and Material from the Base Enemy.
)