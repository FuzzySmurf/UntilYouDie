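; Player character Blueprint that carries a handgun as a child actor and fires it from the Fire input.
; The construction script snaps the Hundgun component to the mesh's WeaponSocket.
; Pressing Fire sets IsShooting, casts the child actor to Handgun and calls FireWeapon once per press.
; Releasing Fire clears IsShooting, and both events print debug strings.
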(event Input|ActionEvents|InputActionFire
  (:Pressed
    (Development|PrintString "AIM")
    (Variables|Default|SetIsShooting? true)
    (bind _ashandgun (Utilities|Casting|CastToHandgun (Variables|/Script/Engine.ChildActorComponent|GetChildActor (Variables|Default|GetHundgun))))
    (Default|FireWeapon _ashandgun))
  (:Released
    (Development|PrintString "STOP" true true "(R=1.000000,G=0.134206,B=0.229912,A=1.000000)")
    (Variables|Default|SetIsShooting? false)))

(fn ConstructionScript
  (Class|SceneComponent|Attachto (Variables|Default|GetHundgun) (Variables|Character|GetMesh) "WeaponSocket" "SnapToTarget" true))